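; BP_EnemyTest is a test enemy that hurts the player on contact and reacts to being hit.
; When a BP_FirstPersonCharacter overlaps its Box component, it applies fixed damage to that character.
; Any damage it takes plays a 2D sound, lowers Health and prints a hit message, or a death message at zero or below, with no destroy or death logic.
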(event OnComponentBeginOverlap(Box)
  (params (OverlappedComponent :type Primitive%20Component%20Object%20Reference) (OtherActor :type Actor%20Object%20Reference) (OtherComp :type Primitive%20Component%20Object%20Reference) (OtherBodyIndex :type Integer) (bFromSweep :type Boolean) (SweepResult :type Hit%20Result%20Structure%20%28by%20ref%29))
  (bind _asbp_first_person_character (Utilities|Casting|CastToBP_FirstPersonCharacter OtherActor))
  (Game|Damage|ApplyDamage _asbp_first_person_character 3e+01 0 0))

(event EventBeginPlay)

(event Collision|EventActorBeginOverlap
  (params (OtherActor :type Actor%20Object%20Reference)))

(event EventTick
  (params (DeltaSeconds :type Float%20%28single-precision%29)))

(event Game|Damage|EventAnyDamage
  (params (Damage :type Float%20%28single-precision%29) (DamageType :type Damage%20Type%20Object%20Reference) (InstigatedBy :type Controller%20Object%20Reference) (DamageCauser :type Actor%20Object%20Reference))
  (Audio|PlaySound2D "/Game/Sounds/SoundSource/Icantbelieve.Icantbelieve" 1.0 1.0 0.0 0 0)
  (bind _output_get (Variables|Default|Sethealth (- (Variables|Default|Gethealth) Damage)))
  (if (<= _output_get 0.0)
    (Development|PrintString "Subject Dead!" true true "(R=1.000000,G=0.867417,B=0.966854,A=1.000000)")
    (else
      (Development|PrintString "Shot Hit!" true true "(R=0.033466,G=1.000000,B=0.000000,A=1.000000)"))))

(fn ConstructionScript)