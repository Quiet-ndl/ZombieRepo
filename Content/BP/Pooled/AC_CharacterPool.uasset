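; AC_CharacterPool is a component that pools characters for reuse.
; On BeginPlay it spawns PoolSize actors of PooledCharClass, owned by the component's owner, and stores each as unused.
; SpawnFromPool finds the first valid free actor by linear search, moves it to the given transform, marks it in use and returns it.
; The pool never grows, and the target location and actor inputs are unused.
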(event Custom|InitializePool
  (for _index (range 0 (Variables|Default|GetPoolSize))
    (bind _returnvalue (Game|SpawnActorfromClass (Variables|Default|GetPooledCharClass) (Math|Transform|MakeTransform "0, 0, 0" "0, 0, 0" "1.000000,1.000000,1.000000") "Undefined" "MultiplyWithRoot" (Components|GetOwner self) 0 0))
    (Utilities|Array|AddUnique (Variables|Default|GetObjectPool) _returnvalue)
    (Default|SetUseFalse _returnvalue)))

(event EventBeginPlay
  (CallFunction|InitializePool))

(fn FindFirstAvailableActor
  (for _array_element (Variables|Default|GetObjectPool)
    (Utilities|IsValid _array_element
      (:Is%20Valid
        (if (not (Variables|/Game/BP/Pooled/BP_PooledCharacter.BP_PooledCharacter_C|GetInUse _array_element))
          (return _array_element))))))

(fn SpawnfromPool
  (params (SpawnTF :type Transform%20%28by%20ref%29) (TargetLocation :type Vector) (TargetActor :type Actor%20Object%20Reference))
  (bind _poolactor (CallFunction|FindFirstAvailableActor))
  (Utilities|IsValid _poolactor
    (:Is%20Valid
      (Transformation|SetActorTransform _poolactor SpawnTF)
      (Default|SetinUse _poolactor true)
      (return _poolactor))))