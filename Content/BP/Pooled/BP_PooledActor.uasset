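; BP_PooledActor is a poolable actor that toggles between active and dormant states instead of being spawned and destroyed.
; SetInUse drives collision, visibility and ticking from one flag, and BeginPlay starts the actor dormant.
; Activation also starts a TimeToLive timer, with SetUseFalse available to switch the actor back to dormant.
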(event Custom|SetUseFalse
  (CallFunction|SetinUse false))

(event Custom|SetInUse
  (params (InUse :type Boolean))
  (Variables|Default|SetInUse InUse)
  (Collision|SetActorEnableCollision InUse)
  (Rendering|SetActorHiddenInGame (not InUse))
  (Actor|Tick|SetActorTickEnabled InUse)
  (if InUse
    (Utilities|Time|SetTimerbyEvent (EventDispatchers|CreateEvent :!event Custom|SetUseFalse) (Variables|Default|GetTimeToLive))))

(event EventBeginPlay
  (CallFunction|SetinUse false))

(event Collision|EventActorBeginOverlap
  (params (OtherActor :type Actor%20Object%20Reference)))

(event EventTick
  (params (DeltaSeconds :type Float%20%28single-precision%29)))

(fn ConstructionScript)