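; BP_PooledCharacter is a poolable actor that is switched on and off for reuse and starts out inactive.
; SetInUse toggles its collision, visibility and tick together, and on activation starts a TimeToLive timer, apparently to deactivate it through SetUseFalse.
; While active it draws a red debug sphere around itself every tick.
; Destroyed also calls SetUseFalse, though this does not prevent destruction, and its parent call is unwired.
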(event Custom|SetUseFalse
  (CallFunction|SetinUse false))

(event Custom|SetInUse
  (params (InUse :type Boolean))
  (Variables|Default|SetInUse InUse)
  (Collision|SetActorEnableCollision InUse)
  (Rendering|SetActorHiddenInGame (not InUse))
  (Actor|Tick|SetActorTickEnabled InUse)
  (if InUse
    (Utilities|Time|SetTimerbyEvent (EventDispatchers|CreateEvent :!event Custom|SetUseFalse) (Variables|Default|GetTimeToLive))))

(event EventBeginPlay
  (CallFunction|SetinUse false))

(event Collision|EventActorBeginOverlap
  (params (OtherActor :type Actor%20Object%20Reference)))

(event EventTick
  (params (DeltaSeconds :type Float%20%28single-precision%29))
  (Rendering|Debug|DrawDebugSphere (Transformation|GetActorLocation) 4e+02 12 "(R=1.000000,G=0.000000,B=0.005894,A=1.000000)" 0.01 1e+01))

(event EventDestroyed
  (CallFunction|SetUseFalse))

(fn ConstructionScript)