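; BP_SpawningTarget is a damageable target that spawns actors from its ACObjectPool component and displays pool usage.
; Each hit adds to TotalDamage and activates a pooled actor with physics at a random navigable point nearby.
; A retriggerable delay debounces recounting of used and unused slots into two text renders.
; Hits reverse a timeline meant to scale the text's X axis, and a timer replays it five seconds after each recount.
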(event Custom|ResetText
  (Components|Timeline|PlayfromStart (Variables|Default|GetTimeline)))

(event EventBeginPlay
  (bind _ac_objectpool (Variables|Default|GetAC_ObjectPool))
  (bind _objectpool (Variables|/Game/BP/Pooled/AC_ObjectPool.AC_ObjectPool_C|GetObjectPool _ac_objectpool))
  (Rendering|Components|TextRender|SetText (Variables|Default|GetTextRender) (Utilities|Text|MakeLiteralText "0"))
  (Rendering|Components|TextRender|SetText (Variables|Default|GetTextRender1) (Utilities|Text|MakeLiteralText "0"))
  (Variables|Default|SetUsedSpawns 0)
  (for _array_element _objectpool
    (if (Variables|/Game/BP/Pooled/BP_PooledActor.BP_PooledActor_C|GetInUse _array_element)
      (Variables|Default|SetUsedSpawns (+ (Variables|Default|GetUsedSpawns) 1))))
  (bind _output_get (Variables|Default|SetUnusedSpawns (- (Utilities|Array|Length _objectpool) (Variables|Default|GetUsedSpawns))))
  (Rendering|Components|TextRender|SetText (Variables|Default|GetTextRender) (Utilities|Text|ToText(Integer) (Variables|Default|GetUsedSpawns)))
  (Rendering|Components|TextRender|SetText (Variables|Default|GetTextRender1) (Utilities|Text|ToText(Integer) _output_get))
  (Utilities|Time|SetTimerbyEvent (delegate Custom|ResetText) 5.0))

(event Collision|EventActorBeginOverlap
  (params (OtherActor :type Actor%20Object%20Reference)))

(event EventTick
  (params (DeltaSeconds :type Float%20%28single-precision%29)))

(event Game|Damage|EventAnyDamage
  (params (Damage :type Float%20%28single-precision%29) (DamageType :type Damage%20Type%20Object%20Reference) (InstigatedBy :type Controller%20Object%20Reference) (DamageCauser :type Actor%20Object%20Reference))
  (bind _ac_objectpool (Variables|Default|GetAC_ObjectPool))
  (bind _objectpool (Variables|/Game/BP/Pooled/AC_ObjectPool.AC_ObjectPool_C|GetObjectPool _ac_objectpool))
  (Utilities|String|Reverse (Variables|Default|GetTimeline))
  (Variables|Default|SetTotalDamage (+ Damage (Variables|Default|GetTotalDamage)))
  (bind _randomlocation (Class|NavigationSystemV1|GetRandomLocationinNavigableRadius (Transformation|GetActorLocation) 2.5e+02 0 0))
  (bind _poolactor (Default|SpawnfromPool (Variables|Default|GetAC_ObjectPool) (Math|Conversions|ToTransform(Vector) _randomlocation) "0, 0, 0"))
  (Physics|SetSimulatePhysics (Variables|/Game/BP/Pooled/BP_PooledActor.BP_PooledActor_C|GetSphere _poolactor) true)
  (Default|SetinUse _poolactor true)
  (Utilities|FlowControl|RetriggerableDelay 0.3)
  (Variables|Default|SetUsedSpawns 0)
  (for _array_element _objectpool
    (if (Variables|/Game/BP/Pooled/BP_PooledActor.BP_PooledActor_C|GetInUse _array_element)
      (Variables|Default|SetUsedSpawns (+ (Variables|Default|GetUsedSpawns) 1))))
  (bind _output_get (Variables|Default|SetUnusedSpawns (- (Utilities|Array|Length _objectpool) (Variables|Default|GetUsedSpawns))))
  (Rendering|Components|TextRender|SetText (Variables|Default|GetTextRender) (Utilities|Text|ToText(Integer) (Variables|Default|GetUsedSpawns)))
  (Rendering|Components|TextRender|SetText (Variables|Default|GetTextRender1) (Utilities|Text|ToText(Integer) _output_get))
  (Utilities|Time|SetTimerbyEvent (delegate Custom|ResetText) 5.0))

(fn ConstructionScript)