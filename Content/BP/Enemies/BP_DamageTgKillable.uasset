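; Killable damage target enemy that displays the latest hit and accumulated damage on two text renders.
; Damage exceeding Health spawns from the spawn manager's coin pool at the mesh transform and destroys the actor.
; Otherwise a retriggerable delay arms a reset timer, which plays a timeline scaling the text's X and clearing the total when finished.
; Each new hit reverses that timeline.
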(event Custom|ResetText
  (Components|Timeline|PlayfromStart (Variables|Default|GetTimeline)))

(event EventBeginPlay
  (Rendering|Components|TextRender|SetText (Variables|Default|GetTextRender) (Utilities|Text|MakeLiteralText (Utilities|Text|ToText(Float) (Variables|Default|GetHealth) "HalfToEven")))
  (bind _returnvalue (Actor|GetActorOfClass "/Game/BP/Objects/BP_SpawnManager.BP_SpawnManager_C"))
  (Variables|Default|SetManager _returnvalue)
  (Rendering|Components|TextRender|SetText (Variables|Default|GetTextRender1) (Utilities|Text|MakeLiteralText "0"))
  (Utilities|Time|SetTimerbyEvent (delegate Custom|ResetText) 1.5))

(event Collision|EventActorBeginOverlap
  (params (OtherActor :type Actor%20Object%20Reference)))

(event EventTick
  (params (DeltaSeconds :type Float%20%28single-precision%29)))

(event Game|Damage|EventAnyDamage
  (params (Damage :type Float%20%28single-precision%29) (DamageType :type Damage%20Type%20Object%20Reference) (InstigatedBy :type Controller%20Object%20Reference) (DamageCauser :type Actor%20Object%20Reference))
  (Utilities|String|Reverse (Variables|Default|GetTimeline))
  (Rendering|Components|TextRender|SetText (Variables|Default|GetTextRender) (Utilities|Text|ToText(Float) Damage "HalfToEven"))
  (bind _output_get (Variables|Default|SetTotalDamage (+ Damage (Variables|Default|GetTotalDamage))))
  (if (> _output_get (Variables|Default|GetHealth))
    (Rendering|Components|TextRender|SetText (Variables|Default|GetTextRender1) (Utilities|Text|MakeLiteralText "Dead"))
    (Default|SpawnfromPool (Variables|/Game/BP/Objects/BP_SpawnManager.BP_SpawnManager_C|GetAC_CoinPool (Variables|Default|GetManager)) (Transformation|GetWorldTransform (Variables|Default|GetStaticMesh)) "0, 0, 0")
    (Actor|DestroyActor)
    (else
      (Rendering|Components|TextRender|SetText (Variables|Default|GetTextRender1) (Utilities|Text|ToText(Float) _output_get "HalfToEven"))
      (Utilities|FlowControl|RetriggerableDelay 0.3)
      (Utilities|Time|SetTimerbyEvent (delegate Custom|ResetText) 1.5))))

(fn ConstructionScript)