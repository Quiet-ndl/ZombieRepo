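; BP_SpawnerTargetVFX is a damage-readout target that displays the last hit and a running total on two text renders.
; Each hit spawns a random spark or fire emitter, updates both texts and reverses a timeline driving their X scale.
; After a retriggerable delay, a timer is set to play that timeline forward, clearing the accumulated total when it finishes.
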(event Custom|ResetText
  (Components|Timeline|PlayfromStart (Variables|Default|GetTimeline)))

(event EventBeginPlay
  (Rendering|Components|TextRender|SetText (Variables|Default|GetTextRender) (Utilities|Text|MakeLiteralText "0"))
  (Rendering|Components|TextRender|SetText (Variables|Default|GetTextRender1) (Utilities|Text|MakeLiteralText "0"))
  (Utilities|Time|SetTimerbyEvent (delegate Custom|ResetText) 1.5))

(event Collision|EventActorBeginOverlap
  (params (OtherActor :type Actor%20Object%20Reference)))

(event EventTick
  (params (DeltaSeconds :type Float%20%28single-precision%29)))

(event Game|Damage|EventAnyDamage
  (params (Damage :type Float%20%28single-precision%29) (DamageType :type Damage%20Type%20Object%20Reference) (InstigatedBy :type Controller%20Object%20Reference) (DamageCauser :type Actor%20Object%20Reference))
  (Effects|SpawnEmitterAttached (select (Math|Random|RandomBool) "/Game/StarterContent/Particles/P_Sparks.P_Sparks" "/Game/StarterContent/Particles/P_Fire.P_Fire") (Variables|Default|GetTextRender1) "None" "0.000000,0.000000,80.000000")
  (Utilities|String|Reverse (Variables|Default|GetTimeline))
  (Rendering|Components|TextRender|SetText (Variables|Default|GetTextRender) (Utilities|Text|ToText(Float) Damage "HalfToEven"))
  (bind _output_get (Variables|Default|SetTotalDamage (+ Damage (Variables|Default|GetTotalDamage))))
  (Rendering|Components|TextRender|SetText (Variables|Default|GetTextRender1) (Utilities|Text|ToText(Float) _output_get "HalfToEven"))
  (Utilities|FlowControl|RetriggerableDelay 0.3)
  (Utilities|Time|SetTimerbyEvent (delegate Custom|ResetText) 1.5))

(fn ConstructionScript)