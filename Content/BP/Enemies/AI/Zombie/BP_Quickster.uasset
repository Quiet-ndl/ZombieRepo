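; Quickster zombie enemy that jumps at its target when attacking and then self-detonates.
; Attack triggers AtkJump and CountdownDeath, which plays a montage and explodes after DeathTime or on blend-out.
; The blast sphere-traces for the player, damages hit components not tagged "Activate", plays a sound, then calls SetUseFalse.
; A looping velocity timer makes it jump when stationary to unstick itself.
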(event Custom|CountdownDeath
  (bind _returnvalue (Transformation|GetActorLocation))
  (Animation|Montage|PlayMontage (Variables|Character|GetMesh) (Variables|Default|GetAttack1M)
    (:then
      (Utilities|FlowControl|RetriggerableDelay (Variables|Default|GetDeathTime)))
    (:OnBlendOut
      _))
  (bind _outhits (Collision|MultiSphereTraceByChannel _returnvalue _returnvalue 3e+02 "TraceTypeQuery1" false 0 "ForDuration"))
  (Audio|PlaySoundatLocation "/Game/Sounds/SoundCue/FastExplode_Cue.FastExplode_Cue" (Transformation|GetActorLocation) "0, 0, 0" 1.0 1.0 0.0 0 0 0 0)
  (bind _array_element (Utilities|Array|ForEachLoopwithBreak _outhits)
    (:LoopBody
      (if (== (.HitActor (Collision|BreakHitResult _array_element)) (Game|GetPlayerCharacter 0))
        (if (not (Components|ComponentHasTag (.HitComponent (Collision|BreakHitResult _array_element)) "Activate"))
          (Game|Damage|ApplyDamage (.HitActor (Collision|BreakHitResult _array_element)) 15.0 0 self))))
    (:Completed
      (Utilities|FlowControl|Delay 0.1)
      (CallFunction|SetUseFalse))))

(event Custom|Unstick
  (Utilities|FlowControl|Delay 1.0)
  (Utilities|Time|SetTimerbyEvent (delegate Custom|Velocity) 0.5 true))

(event Custom|Velocity
  (if (Utilities|Operators|EqualEqual :A (Variables|/Script/Engine.MovementComponent|GetVelocity (Variables|Character|GetCharacterMovement)) :ErrorTolerance 1.0)
    (CallFunction|AtkJump)
    (CallFunction|Unstick)))

(event EventBeginPlay
  (|CallParentFunction)
  (CallFunction|Unstick))

(event Collision|EventActorBeginOverlap
  (params (OtherActor :type Actor%20Object%20Reference))
  (|CallParentFunction OtherActor) ; This node is disabled and will not be called.\nDrag off pins to build functionality.
)

(event EventTick
  (params (DeltaSeconds :type Float%20%28single-precision%29))
  (|CallParentFunction DeltaSeconds) ; This node is disabled and will not be called.\nDrag off pins to build functionality.
)

(event Game|Damage|EventAnyDamage
  (params (Damage :type Float%20%28single-precision%29) (DamageType :type Damage%20Type%20Object%20Reference) (InstigatedBy :type Controller%20Object%20Reference) (DamageCauser :type Actor%20Object%20Reference))
  (|CallParentFunction Damage DamageType InstigatedBy DamageCauser))

(event EventAttack
  (CallFunction|AtkJump)
  (CallFunction|CountdownDeath))

(fn ConstructionScript
  (|CallParentFunction))