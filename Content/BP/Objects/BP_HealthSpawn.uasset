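; Health pickup spawn point that places a pooled health actor just above its Cube at BeginPlay.
; It finds BP_SpawnManager and draws from its health pool component instead of spawning directly, then binds to the spawned actor's begin-overlap event.
; When the player character overlaps that actor, a randomly delayed timer of 15 to 45 seconds starts, apparently to respawn health.
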(event Custom|OnActorBeginOverlap_Event
  (params (OverlappedActor :type Actor%20Object%20Reference) (OtherActor :type Actor%20Object%20Reference))
  (if (== OtherActor (Game|GetPlayerCharacter 0))
    (Utilities|Time|SetTimerbyEvent (EventDispatchers|CreateEvent :!event Custom|Spawn%20New%20Health) (Math|Random|RandomFloatinRange 15.0 45.0))))

(event Custom|Spawn%20New%20Health
  (bind _poolactor (Default|SpawnfromPool (Variables|/Game/BP/Objects/BP_SpawnManager.BP_SpawnManager_C|GetAC_HealthPool (Variables|Default|GetManager)) (Math|Conversions|ToTransform(Vector) (+ (.location (Transformation|GetWorldTransform (Variables|Default|GetCube))) "0.000000,0.000000,30.000000")) "0, 0, 0"))
  (Utilities|IsValid _poolactor
    (:Is%20Valid
      (EventDispatchers|AssignOnActorBeginOverlap _poolactor (delegate Custom|OnActorBeginOverlap_Event)))))

(event EventBeginPlay
  (bind _returnvalue (Actor|GetActorOfClass "/Game/BP/Objects/BP_SpawnManager.BP_SpawnManager_C"))
  (Variables|Default|SetManager _returnvalue)
  (CallFunction|SpawnNewHealth))

(event EventTick
  (params (DeltaSeconds :type Float%20%28single-precision%29)))

(fn ConstructionScript)