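; Zombie director that runs wave spawning for Survival, Endless and Objective game modes.
; DirectorUpdate sets target count, interval, distance band and special chance, which NextWave scales by wave number.
; A timer triggers passes over active BP_ZombieSpawn points within that band of the player, up to the target.
; Survival and Objective advance after a delay, while Endless uses a check timer to wait until the zombie count reaches zero.
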(event Custom|SpawnZombiesAtPoints
  (bind _array_element (Utilities|Array|ForEachLoopwithBreak (Variables|Refs|GetSpawnpoints) :!label _label)
    (:LoopBody
      (if (< (Variables|DirectorValues|GetZombiesCurrent) (Variables|DirectorValues|GetZombiesDesired))
        (if (Math|Boolean|ANDBoolean (< (CallFunction|DistCheck _array_element (Game|GetPlayerCharacter 0)) (Variables|DirectorValues|GetMaxDist)) (> (CallFunction|DistCheck _array_element (Game|GetPlayerCharacter 0)) (Variables|DirectorValues|GetMinDist)) (Variables|/Game/BP/Objects/BP_ZombieSpawn.BP_ZombieSpawn_C|GetActive _array_element))
          (Utilities|IsValid _array_element
            (:Is%20Valid
              (Variables|/Game/BP/Objects/BP_ZombieSpawn.BP_ZombieSpawn_C|SetSpecialChance _array_element (Variables|DirectorValues|GetSpecial%20Chance))
              (Default|SpawnZom _array_element)
              (Development|PrintString "Zed Spawned" true true "(R=0.005274,G=0.182292,B=0.000000,A=1.000000)" 1.0)
              (CallFunction|EditZombies false)
              (Development|PrintString (Utilities|String|Append "NewZValue-" (Utilities|String|ToString(Integer) (Variables|DirectorValues|GetZombiesCurrent)))))))
        (else
          (CallFunction|StopZombies)
          (goto _label Break))))
    (:Completed
      (switch Utilities|FlowControl|Switch|SwitchonGamemode (Variables|0-Public|GetGamemode)
        (:NewEnumerator0
          (Variables|DirectorValues|SetZombieMin (* 1 (/ (Variables|DirectorValues|GetWaveNum) 2)) :!label _label_2)
          (bind _result (Math|Integer|IncrementInt (Variables|DirectorValues|GetWaveNum))
            (:%20%20
              (CallFunction|StopZombies)
              (Utilities|FlowControl|Delay (Math|Float|Clamp(Float) (* (CallFunction|CalcDelay) 2.0) 1.0 2e+01))
              (CallFunction|NextWave)
              (Development|PrintString (Utilities|String|Append "WAVE-" (Utilities|String|ToString(Integer) _result))))))
        (:NewEnumerator1
          (CallFunction|StopZombies)
          (bind _returnvalue (Utilities|Time|SetTimerbyEvent (EventDispatchers|CreateEvent :!event Custom|CheckCurrentZombies) 1.0 true true))
          (Variables|Refs|SetZCheckTimer _returnvalue))
        (:NewEnumerator2
          (goto _label_2))))))

(event Custom|StartTimers
  (bind _returnvalue (Utilities|Time|SetTimerbyEvent (delegate Custom|SpawnZombiesAtPoints) (Variables|DirectorValues|GetTimeBetweenZs) true))
  (Variables|Refs|SetZSpawnTimer _returnvalue))

(event Custom|StopZombies
  (bind _zspawntimer (Variables|Refs|GetZSpawnTimer))
  (if (Utilities|Time|IsValidTimerHandle _zspawntimer)
    (Utilities|Time|ClearandInvalidateTimerbyHandle _zspawntimer)))

(event Custom|CheckCurrentZombies
  (bind _zombiescurrent (Variables|DirectorValues|GetZombiesCurrent))
  (if (<= _zombiescurrent 0)
    (Math|Integer|IncrementInt (Variables|DirectorValues|GetWaveNum)
      (:%20%20
        (Utilities|FlowControl|Delay (CallFunction|CalcDelay))
        (CallFunction|NextWave)))
    (else
      (Development|PrintString (Utilities|String|Append (Utilities|String|ToString(Integer) _zombiescurrent) " Zeds Remain") true true "(R=1.000000,G=0.135502,B=0.000000,A=1.000000)" 1.0))))

(event Custom|NextWave
  (bind _wavenum (Variables|DirectorValues|GetWaveNum))
  (bind _returnvalue (Math|Conversions|ToFloat(Integer) _wavenum))
  (bind _returnvalue_2 (/ _returnvalue 3.0))
  (Utilities|Time|ClearandInvalidateTimerbyHandle (Variables|Refs|GetZCheckTimer))
  (Variables|DirectorValues|SetZombiesCurrent 0)
  (CallFunction|DirectorUpdate (Math|Integer|Clamp(Integer) (* (* (Variables|DirectorValues|GetZombieMin) _wavenum) (Math|Integer|SelectInt 3 1 (> _wavenum 10))) 4 55) (Math|Float|Clamp(Float) (Math|Float|Clamp(Float) (/ 5.0 _returnvalue) 0.2 5.0) 0.2 4.0) (Math|Float|Clamp(Float) (/ 2.5e+02 _returnvalue_2) 1.5e+02 5e+02) (Math|Float|Clamp(Float) (* 5e+02 _returnvalue_2) 4.5e+02 1.85e+03) (/ 1.0 (/ _returnvalue 2e+01)))
  (CallFunction|StartTimers)
  (Development|PrintString (Utilities|String|Append "Wave-" (Utilities|String|ToString(Integer) (Variables|DirectorValues|GetWaveNum))) true true "(R=1.000000,G=0.135502,B=0.000000,A=1.000000)" 1.0))

(event EventBeginPlay
  (bind _outactors (Actor|GetAllActorsOfClass "/Game/BP/Objects/BP_ZombieSpawn.BP_ZombieSpawn_C"))
  (Variables|Refs|SetSpawnpoints _outactors)
  (Utilities|FlowControl|Delay (Variables|0-Public|GetStartDelay))
  (switch Utilities|FlowControl|Switch|SwitchonGamemode (Variables|0-Public|GetGamemode)
    (:NewEnumerator0
      (CallFunction|DirectorUpdate (Math|Random|RandomIntegerinRange (Variables|DirectorValues|GetZombieMin) 8) 0.25 2.5e+02 1.5e+03 0.9 :!label _label)
      ;[0.15 0.15 0.15 0.5] Occasional gaps in zombie spawn
      (CallFunction|StartTimers))
    (:NewEnumerator1
      (CallFunction|DirectorUpdate (Math|Random|RandomIntegerinRange (Variables|DirectorValues|GetZombieMin) 8) 2.0 2.5e+02 8e+02 0.95)
      (CallFunction|NextWave))
    (:NewEnumerator2
      (goto _label))))

(fn ConstructionScript)

(fn DistCheck
  (params (Target :type Actor%20Object%20Reference) (Target1 :type Actor%20Object%20Reference))
  (return (Math|Vector|Distance(Vector) (Transformation|GetActorLocation Target) (Transformation|GetActorLocation Target1))))

(fn DirectorUpdate
  (params (DesiredZombies :type Integer) (SpawnInterval :type Float%20%28double-precision%29) (MinSpawnDistance :type Float%20%28double-precision%29) (MaxSpawnDistance :type Float%20%28double-precision%29) (Special%20Chance :type Float%20%28single-precision%29))
  (Variables|DirectorValues|SetZombiesDesired DesiredZombies)
  (Variables|DirectorValues|SetTimeBetweenZs SpawnInterval)
  (Variables|DirectorValues|SetMinDist MinSpawnDistance)
  (Variables|DirectorValues|SetMaxDist MaxSpawnDistance)
  (Variables|DirectorValues|SetSpecial%20Chance Special%20Chance))

(fn Check/SetZombies
  (bind _zombiescurrent (Variables|DirectorValues|GetZombiesCurrent))
  (bind _outactors (Actor|GetAllActorsOfClass "/Game/BP/Enemies/AI/Zombie/BP_ZombieBase.BP_ZombieBase_C"))
  (for _array_element _outactors
    (if (Variables|/Game/BP/Pooled/BP_PooledCharacter.BP_PooledCharacter_C|GetInUse _array_element)
      (Math|Integer|IncrementInt _zombiescurrent)))
  (return _zombiescurrent))

(fn CalcDelay
  (return (Math|Conversions|ToFloat(Integer) (Math|Integer|Clamp(Integer) (* (Variables|DirectorValues|GetWaveNum) 5) 0 35))))

(fn EditZombies
  (params (Negate :type Boolean))
  (if Negate
    (Variables|DirectorValues|SetZombiesCurrent (- (Variables|DirectorValues|GetZombiesCurrent) 1))
    (else
      (Variables|DirectorValues|SetZombiesCurrent (+ (Variables|DirectorValues|GetZombiesCurrent) 1))))
  (return (Variables|DirectorValues|GetZombiesCurrent)))