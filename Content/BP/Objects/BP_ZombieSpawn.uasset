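; Zombie spawn point that draws enemies from the zombie manager's object pools and targets them at the player.
; SpawnZom makes a SpecialChance roll for the regular pool, otherwise the big-zombie pool, then after a short delay activates and teleports the zombie above itself.
; Each death calls EditZombies on the manager.
; A cylinder overlap clears the Active flag while the player is inside, though SpawnZom never checks it.
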(event OnComponentBeginOverlap(Cylinder)
  (params (OverlappedComponent :type Primitive%20Component%20Object%20Reference) (OtherActor :type Actor%20Object%20Reference) (OtherComp :type Primitive%20Component%20Object%20Reference) (OtherBodyIndex :type Integer) (bFromSweep :type Boolean) (SweepResult :type Hit%20Result%20Structure%20%28by%20ref%29))
  (if (== OtherActor (Game|GetPlayerCharacter 0))
    (Variables|Default|SetActive false)))

(event OnComponentEndOverlap(Cylinder)
  (params (OverlappedComponent :type Primitive%20Component%20Object%20Reference) (OtherActor :type Actor%20Object%20Reference) (OtherComp :type Primitive%20Component%20Object%20Reference) (OtherBodyIndex :type Integer))
  (if (== OtherActor (Game|GetPlayerCharacter 0))
    (Variables|Default|SetActive true)))

(event Custom|SpawnZom
  (bind _returnvalue (Transformation|GetActorLocation))
  (bind _returnvalue_2 (Game|GetPlayerCharacter 0))
  (bind _manager (Variables|Default|GetManager))
  (bind _returnvalue_3 (+ _returnvalue "0.000000,0.000000,170.000000"))
  (if (Math|Random|RandomBoolwithWeight (Variables|Default|GetSpecialChance))
    (bind _poolactor (Default|SpawnfromPool (Variables|/Game/BP/Objects/BP_ZombieManager.BP_ZombieManager_C|GetAC_ZombiePool _manager) (Math|Transform|MakeTransform _returnvalue_3 "0, 0, 0" "1.000000,1.000000,1.000000") "0, 0, 0" _returnvalue_2))
    (Utilities|FlowControl|Delay 0.2)
    (Utilities|IsValid _poolactor
      (:Is%20Valid
        (EventDispatchers|AssignOnDeath _poolactor (delegate Custom|OnDeath_Event))
        (Default|SetinUse _poolactor true)
        (Transformation|SetActorLocation _poolactor _returnvalue_3 false false)))
    (else
      (bind _poolactor_2 (Default|SpawnfromPool (Variables|/Game/BP/Objects/BP_ZombieManager.BP_ZombieManager_C|GetAC_BigZombiePool1 _manager) (Math|Transform|MakeTransform _returnvalue_3 "0, 0, 0" "1.000000,1.000000,1.000000") "0, 0, 0" _returnvalue_2))
      (Utilities|FlowControl|Delay 0.2)
      (Utilities|IsValid _poolactor_2
        (:Is%20Valid
          (EventDispatchers|AssignOnDeath _poolactor_2 (delegate Custom|OnDeath_Event))
          (Default|SetinUse _poolactor_2 true)
          (Transformation|SetActorLocation _poolactor_2 _returnvalue_3 false false))))))

(event Custom|OnDeath_Event
  (Default|EditZombies (Variables|Default|GetManager) true)
  (Development|PrintString "ZOMBIE KILLED" true true "(R=1.000000,G=0.994037,B=0.947917,A=1.000000)"))

(event EventBeginPlay
  (bind _returnvalue (Actor|GetActorOfClass "/Game/BP/Objects/BP_ZombieManager.BP_ZombieManager_C"))
  (Variables|Default|SetManager _returnvalue))

(fn ConstructionScript)