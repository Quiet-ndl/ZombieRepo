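; BP_HealthPickup is a pickup actor that adds a health pack to the first-person player character.
; It caches the character on BeginPlay and responds when that character overlaps its Box.
; Below the three-pack cap, it increments and clamps the count, then calls SetInUse(false) to take itself out of use.
; A two-part click sound follows, with randomized pitch first and a higher, louder repeat after a short delay.
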(event OnComponentBeginOverlap(Box)
  (params (OverlappedComponent :type Primitive%20Component%20Object%20Reference) (OtherActor :type Actor%20Object%20Reference) (OtherComp :type Primitive%20Component%20Object%20Reference) (OtherBodyIndex :type Integer) (bFromSweep :type Boolean) (SweepResult :type Hit%20Result%20Structure%20%28by%20ref%29))
  (if (== OtherActor (Variables|Default|GetAs%20BP%20First%20Person%20Character))
    (if (not (== (Variables|/Game/FirstPerson/Blueprints/BP_FirstPersonCharacter.BP_FirstPersonCharacter_C|GetHealthPacks (Variables|Default|GetAs%20BP%20First%20Person%20Character)) 3))
      (bind _result (Math|Integer|IncrementInt (Variables|/Game/FirstPerson/Blueprints/BP_FirstPersonCharacter.BP_FirstPersonCharacter_C|GetHealthPacks (Variables|Default|GetAs%20BP%20First%20Person%20Character)))
        (:%20%20
          (Variables|/Game/FirstPerson/Blueprints/BP_FirstPersonCharacter.BP_FirstPersonCharacter_C|SetHealthPacks (Variables|Default|GetAs%20BP%20First%20Person%20Character) (Math|Integer|Clamp(Integer) _result 0 3))
          (CallFunction|SetinUse false)
          (Audio|PlaySound2D "/Engine/VREditor/Sounds/UI/Click_on_Button.Click_on_Button" 1.0 (Math|Random|RandomFloatinRange 0.9 1.0) 0.0 0 0)
          (Utilities|FlowControl|Delay 0.2)
          (Audio|PlaySound2D "/Engine/VREditor/Sounds/UI/Click_on_Button.Click_on_Button" 1.1 1.2 0.0 0 0))))))

(event EventBeginPlay
  (bind _asbp_first_person_character (Utilities|Casting|CastToBP_FirstPersonCharacter (Game|GetPlayerCharacter 0)))
  (Variables|Default|SetAs%20BP%20First%20Person%20Character _asbp_first_person_character))

(event Collision|EventActorBeginOverlap
  (params (OtherActor :type Actor%20Object%20Reference)))

(event EventTick
  (params (DeltaSeconds :type Float%20%28single-precision%29)))

(fn ConstructionScript)