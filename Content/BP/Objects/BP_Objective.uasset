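; BP_Objective is an objective actor that loses health when zombies attack it.
; Its AnyDamage event ignores damage causers that are not BP_ZombieBase, plays a randomly pitched bell sound and subtracts the damage from Health.
; Losing health and reaching zero are only reported through debug print strings, with no further game-over or destruction logic.
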(event EventBeginPlay)

(event Collision|EventActorBeginOverlap
  (params (OtherActor :type Actor%20Object%20Reference)))

(event EventTick
  (params (DeltaSeconds :type Float%20%28single-precision%29)))

(event Game|Damage|EventAnyDamage
  (params (Damage :type Float%20%28single-precision%29) (DamageType :type Damage%20Type%20Object%20Reference) (InstigatedBy :type Controller%20Object%20Reference) (DamageCauser :type Actor%20Object%20Reference))
  (Utilities|Casting|CastToBP_ZombieBase DamageCauser)
  (Audio|PlaySound2D "/Game/ObjectAssets/Sounds/ElectroBell.ElectroBell" 1.0 (Math|Random|RandomFloatinRange 0.9 1.1) 0.0 0 0)
  (bind _output_get (Variables|Default|Sethealth (- (Variables|Default|Gethealth) Damage)))
  (if (<= _output_get 0.0)
    (Development|PrintString "ObjectiveLost" true true "(R=1.000000,G=0.000000,B=0.068094,A=1.000000)")
    (else
      (Development|PrintString (Utilities|String|Append "ObjectiveLostHP" (Utilities|String|ToString(Float) Damage)) true true "(R=1.000000,G=0.000000,B=0.068094,A=1.000000)"))))

(fn ConstructionScript)